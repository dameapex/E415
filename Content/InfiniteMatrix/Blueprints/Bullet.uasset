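; Bullet is a projectile actor that flies forward along world X and removes itself after a short lifetime.
; Each tick it reads the player's current ForwardSpeed, adds a fixed offset, and moves by a swept world offset, so it always outpaces the player.
; A hit on its static mesh destroys it only when the other actor is a BP_Tunnel.
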(event `self.ReceiveBeginPlay`
  (`KismetSystemLibrary.Delay` 3.0)
  (`self.K2_DestroyActor`))

(event `self.ReceiveTick`
  (params (DeltaSeconds :type "Float (single-precision)"))
  (bind _asbp_player (cast `/Game/InfiniteMatrix/Blueprints/BP_Player` (`GameplayStatics.GetPlayerPawn` 0)))
  (`self.K2_AddActorWorldOffset` (`KismetMathLibrary.MakeVector` (* (+ (`/Game/InfiniteMatrix/Blueprints/BP_Player.ForwardSpeed` _asbp_player) 3000.0) DeltaSeconds)) true))

(event `self.StaticMeshComponent.OnComponentHit`
  (params (HitComponent :type "PrimitiveComponent Object Reference") (OtherActor :type "Actor Object Reference") (OtherComp :type "PrimitiveComponent Object Reference") (NormalImpulse :type "Vector Structure") (Hit :type "HitResult Structure (by ref)"))
  (cast `/Game/InfiniteMatrix/Blueprints/BP_Tunnel` OtherActor)
  (`self.K2_DestroyActor`))

(fn `UserConstructionScript`)