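; BP_Tunnel is an infinite-runner tunnel segment with a spinning holed wall, health pack and enemy.
; Crossing its trigger scores if the wall went untouched, asks TunnelSpawner for another tunnel, then destroys this one.
; Wall (once) and enemy hits damage the player, possibly fatally; bullets destroy enemies and health packs heal.
; Randomize functions, not called here, pick meshes, with empty options for pack and enemy, and wall roll.
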(event `self.ReceiveBeginPlay`)

(event `self.ReceiveTick`
  (params (DeltaSeconds :type "Float (single-precision)"))
  (bind _returnvalue (* DeltaSeconds (`self.HPRotateSpeed`)))
  (`SceneComponent.K2_AddLocalRotation` (`self.WallMesh`) (`KismetMathLibrary.MakeRotator` (* DeltaSeconds (`self.RotateSpeed`))) false false)
  (`SceneComponent.K2_AddLocalRotation` (`self.HealthPack`) (`KismetMathLibrary.MakeRotator` _returnvalue 0.0 _returnvalue) false false)
  (`SceneComponent.K2_AddLocalRotation` (`self.Enermy`) (`KismetMathLibrary.MakeRotator` (* (`self.EnermyRotationSpeed`) DeltaSeconds)) false false))

(event `self.TriggerZone.OnComponentBeginOverlap`
  (params (OverlappedComponent :type "PrimitiveComponent Object Reference") (OtherActor :type "Actor Object Reference") (OtherComp :type "PrimitiveComponent Object Reference") (OtherBodyIndex :type Integer) (bFromSweep :type Boolean) (SweepResult :type "HitResult Structure (by ref)"))
  (bind _asbp_player (cast `/Game/InfiniteMatrix/Blueprints/BP_Player` OtherActor))
  (if (`self.CanDamage`)
    (set `/Game/InfiniteMatrix/Blueprints/BP_Player.Score` (+ (`/Game/InfiniteMatrix/Blueprints/BP_Player.Score` _asbp_player) 10) _asbp_player))
  (`/Game/InfiniteMatrix/Blueprints/BP_TunnelSpawner.SpawnTunnelAtSpawnPoint` (`self.TunnelSpawner`))
  (`self.K2_DestroyActor`))

(event `self.WallMesh.OnComponentHit`
  (params (HitComponent :type "PrimitiveComponent Object Reference") (OtherActor :type "Actor Object Reference") (OtherComp :type "PrimitiveComponent Object Reference") (NormalImpulse :type "Vector Structure") (Hit :type "HitResult Structure (by ref)"))
  (bind _asbp_player (cast `/Game/InfiniteMatrix/Blueprints/BP_Player` OtherActor))
  (if (`self.CanDamage`)
    (set `self.CanDamage` false)
    (bind _output_get (set `/Game/InfiniteMatrix/Blueprints/BP_Player.CurrentHealth` (- (`/Game/InfiniteMatrix/Blueprints/BP_Player.CurrentHealth` _asbp_player) 20.0) _asbp_player))
    (if (<= _output_get 0.0)
      (set `/Game/InfiniteMatrix/Blueprints/BP_Player.IsDead` true _asbp_player)
      (`/Game/InfiniteMatrix/Blueprints/BP_Player.DisplayRestart` _asbp_player))))

(event `self.HealthPack.OnComponentBeginOverlap`
  (params (OverlappedComponent :type "PrimitiveComponent Object Reference") (OtherActor :type "Actor Object Reference") (OtherComp :type "PrimitiveComponent Object Reference") (OtherBodyIndex :type Integer) (bFromSweep :type Boolean) (SweepResult :type "HitResult Structure (by ref)"))
  (bind _asbp_player (cast `/Game/InfiniteMatrix/Blueprints/BP_Player` OtherActor))
  (bind _currenthealth (`/Game/InfiniteMatrix/Blueprints/BP_Player.CurrentHealth` _asbp_player))
  (if (< _currenthealth 100.0)
    (set `/Game/InfiniteMatrix/Blueprints/BP_Player.CurrentHealth` (+ _currenthealth 20.0) _asbp_player)))

(event `self.Enermy.OnComponentHit`
  (params (HitComponent :type "PrimitiveComponent Object Reference") (OtherActor :type "Actor Object Reference") (OtherComp :type "PrimitiveComponent Object Reference") (NormalImpulse :type "Vector Structure") (Hit :type "HitResult Structure (by ref)"))
  (bind _asbp_player (cast `/Game/InfiniteMatrix/Blueprints/BP_Player` OtherActor)
    (:`then`
      (bind _output_get (set `/Game/InfiniteMatrix/Blueprints/BP_Player.CurrentHealth` (- (`/Game/InfiniteMatrix/Blueprints/BP_Player.CurrentHealth` _asbp_player) 20.0) _asbp_player))
      (`ActorComponent.K2_DestroyComponent` (`self.enermy`))
      (if (<= _output_get 0.0)
        (set `/Game/InfiniteMatrix/Blueprints/BP_Player.IsDead` true _asbp_player)
        (`/Game/InfiniteMatrix/Blueprints/BP_Player.DisplayRestart` _asbp_player)))
    (:`CastFailed`
      (bind _asbullet (cast `/Game/InfiniteMatrix/Blueprints/Bullet` OtherActor))
      (`ActorComponent.K2_DestroyComponent` (`self.enermy`))
      (`/Engine/EditorBlueprintResources/StandardMacros.IsValid` _asbullet
        (:`Is Valid`
          (`self.K2_DestroyActor` _asbullet))))))

(fn `RandomizeEnermy`
  (`StaticMeshComponent.SetStaticMesh` (`self.enermy`) (select `int` (`KismetMathLibrary.RandomIntegerInRange` 0 3) :`0` "/Game/InfiniteMatrix/Meshes/cc0_ufo/StaticMeshes/cc0_ufo.cc0_ufo" :`1` "/Game/InfiniteMatrix/Meshes/dino/StaticMeshes/dino.dino" :`2` null :`3` null :!type "StaticMesh Object Reference")))

(fn `RandomizeHP`
  (`StaticMeshComponent.SetStaticMesh` (`self.HealthPack`) (select `int` (`KismetMathLibrary.RandomIntegerInRange` 0 3) :`0` "/Game/InfiniteMatrix/Meshes/Collectable_Heart_01.Collectable_Heart_01" :`1` null :`2` null :`3` null :!type "StaticMesh Object Reference")))

(fn `RandomizeWall`
  (`StaticMeshComponent.SetStaticMesh` (`self.WallMesh`) (select `int` (`KismetMathLibrary.RandomIntegerInRange` 0 3) :`0` "/Game/InfiniteMatrix/Meshes/SM_Hole_01.SM_Hole_01" :`1` "/Game/InfiniteMatrix/Meshes/SM_Hole_02.SM_Hole_02" :`2` "/Game/InfiniteMatrix/Meshes/SM_Hole_03.SM_Hole_03" :`3` "/Game/InfiniteMatrix/Meshes/SM_Hole_04.SM_Hole_04" :!type "StaticMesh Object Reference"))
  (`SceneComponent.K2_AddLocalRotation` (`self.WallMesh`) (`KismetMathLibrary.MakeRotator` (`KismetMathLibrary.RandomFloatInRange` 0.0 360.0)) false false))

(fn `UserConstructionScript`)